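; Player controller that creates the main UI and handles player-side dialogue input.
; On BeginPlay it adds B_MainUI to the viewport and hands DialogueManager a hardcoded set of Turkish lines attributed to the player pawn.
; Interact presses look up the main UI by class and forward to its dialogue panel.
; EnterDialogue and ExitDialogue disable and re-enable input on the controlled pawn.
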(event EventBeginPlay
  (bind _returnvalue (Game|Player|GetPlayerPawn 0))
  (bind _returnvalue_2 (UserInterface|CreateWidget "/Game/Blueprints/UI/B_MainUI.B_MainUI_C" self))
  (UserInterface|Viewport|AddtoViewport _returnvalue_2 0)
  (Default|SetDialogueDataList (Variables|Default|GetDialogueManager) (Utilities|Array|MakeArray (Utilities|Struct|MakeDialogueData "Metin" _returnvalue "Tamam canım. Heyecanla seni bekliyorum" 0.0) (Utilities|Struct|MakeDialogueData "Metin" _returnvalue "Aferin amk" 0.0))))

(event EventTick
  (params (DeltaSeconds :type Float%20%28single-precision%29)))

(event Input|ActionEvents|InputActionPause
  (params (Key :type Key%20Structure :default "None")))

(event Input|ActionEvents|InputActionInteract
  (params (Key :type Key%20Structure :default "None"))
  (:Pressed
    (bind _foundwidgets (Widget|GetAllWidgetsOfClass "/Game/Blueprints/UI/B_MainUI.B_MainUI_C" true))
    (Default|OnPlayerInteractPressed (Variables|/Game/Blueprints/UI/B_MainUI.B_MainUI_C|GetB_DialoguePanel (Utilities|Array|Get(acopy) _foundwidgets)))))

(fn ConstructionScript)

(fn EnterDialogue
  (Input|DisableInput (Pawn|GetControlledPawn) self))

(fn ExitDialogue
  (Input|EnableInput (Pawn|GetControlledPawn) self))