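; B_InteractionVolume is an overlap volume that makes itself the current interaction target of actors entering it.
; On begin overlap it writes itself to InteractionTarget on the other actor's B_Interactor component, ignoring actors without one.
; On end overlap it clears that target without checking whether it still points to this volume.
; GetName exposes the volume's Name variable.
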(event EventBeginPlay)

(event Collision|EventActorBeginOverlap
  (params (OtherActor :type Actor%20Object%20Reference))
  (Utilities|TrySetInteractableOfTarget OtherActor self))

(event Collision|EventActorEndOverlap
  (params (OtherActor :type Actor%20Object%20Reference))
  (Utilities|TrySetInteractableOfTarget OtherActor))

(fn ConstructionScript)

(fn GetName
  (return (Variables|Default|GetName)))