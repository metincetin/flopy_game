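; B_Jumper is a launcher actor that periodically flings whatever overlaps its box.
; A Delay on Tick calls Jump roughly every two seconds, which scans the box's overlapping actors.
; Physics-simulating primitives, or otherwise character movement components, receive a mass-independent velocity-change impulse from GetTargetVelocity.
; That function holds a normalized RelativeDirection times Force calculation, shown as unused.
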(event EventBeginPlay)

(event Collision|EventActorBeginOverlap
  (params (OtherActor :type Actor%20Object%20Reference)))

(event EventTick
  (params (DeltaSeconds :type Float%20%28single-precision%29))
  (Utilities|FlowControl|Delay 2.0)
  (CallFunction|Jump))

(fn ConstructionScript)

(fn Jump
  (for _array_element (Collision|GetOverlappingActors (Variables|Default|GetBox) 0 :!class /Script/Engine.PrimitiveComponent)
    (if (Physics|IsSimulatingPhysics (Actor|GetComponentbyClass _array_element "/Script/Engine.PrimitiveComponent") "None")
      (Physics|AddImpulse (Actor|GetComponentbyClass _array_element "/Script/Engine.PrimitiveComponent") (Utilities|GetTargetVelocity) "None" true)
      (else
        (Utilities|IsValid (Actor|GetComponentbyClass _array_element "/Script/Engine.CharacterMovementComponent")
          (:Is%20Valid
            (Physics|AddImpulse (Actor|GetComponentbyClass _array_element "/Script/Engine.CharacterMovementComponent") (Utilities|GetTargetVelocity) true)))))))