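; B_Fan is a scene object fan that spins its blades and toggles a Niagara effect while active.
; Each tick, if IsActive is set, it yaws the Blades component by RotationRate scaled by delta time for frame-rate independent spin.
; It also syncs the Niagara component's active state to IsActive every tick, without resetting it.
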(event EventBeginPlay)

(event EventTick
  (params (DeltaSeconds :type Float%20%28single-precision%29))
  (|CallParentFunction DeltaSeconds)
  (Utilities|FlowControl|Sequence
    (:then_0
      (if (Variables|Default|GetisActive)
        (Transformation|AddLocalRotation (Variables|Default|GetBlades) (Math|Rotator|MakeRotator 0.0 0.0 (* DeltaSeconds (Variables|Default|GetRotationRate))) false false)))
    (:then_1
      (Components|Activation|SetActive (Variables|Default|GetNiagara) (Variables|Default|GetisActive) false))))

(fn ConstructionScript)