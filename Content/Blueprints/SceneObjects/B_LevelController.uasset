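; B_LevelController is a scene actor that completes a level objective once the player has collected enough data.
; Until completed, it polls the player controller's CollectedData against RequiredData every Tick.
; On reaching the threshold it latches IsCompleted and calls OnInteract on each of its own B_Driver_Interactable_Behaviour components, passing the player controller's B_Interactor as the instigator.
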(event EventBeginPlay)

(event Collision|EventActorBeginOverlap
  (params (OtherActor :type Actor%20Object%20Reference)))

(event EventTick
  (params (DeltaSeconds :type Float%20%28single-precision%29))
  (bind _returnvalue (Game|GetPlayerController 0))
  (if (not (Variables|Default|GetisCompleted))
    (bind _asb_player_controller (Utilities|Casting|CastToB_PlayerController _returnvalue))
    (if (>= (Variables|/Game/Blueprints/B_PlayerController.B_PlayerController_C|GetcollectedData _asb_player_controller) (Variables|Default|GetrequiredData))
      (Variables|Default|SetisCompleted true)
      (for _array_element (Actor|GetComponentsByClass "/Game/Blueprints/Interaction/Interactables/B_Driver_Interactable_Behaviour.B_Driver_Interactable_Behaviour_C")
        (Default|OnInteract _array_element (Actor|GetComponentbyClass _returnvalue "/Game/Blueprints/Interaction/B_Interactor.B_Interactor_C"))))))

(fn ConstructionScript)