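; B_Pusher is an actor that continuously pushes whatever overlaps it along its forward direction.
; Each tick it applies a velocity-change impulse of PushPower scaled by delta time, so mass is ignored.
; Physics-simulating primitive components receive the impulse directly, while other actors receive it through their CharacterMovementComponent.
; The construction script inverse-scales the Arrow by the actor's scale, keeping its size constant when the actor is resized.
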(event EventBeginPlay)

(event Collision|EventActorBeginOverlap
  (params (OtherActor :type Actor%20Object%20Reference)))

(event EventTick
  (params (DeltaSeconds :type Float%20%28single-precision%29))
  (bind _returnvalue (Transformation|GetActorRotation))
  (bind _pushpower (Variables|Default|GetPushPower))
  (bind _returnvalue_2 (Math|Vector|GetForwardVector _returnvalue))
  (bind _returnvalue_3 (* DeltaSeconds _pushpower))
  (bind _returnvalue_4 (* _returnvalue_2 _returnvalue_3))
  (for _array_element (Collision|GetOverlappingActors 0 :!class /Script/Engine.Actor)
    (if (Physics|IsSimulatingPhysics (Actor|GetComponentbyClass _array_element "/Script/Engine.PrimitiveComponent") "None")
      (Physics|AddImpulse (Actor|GetComponentbyClass _array_element "/Script/Engine.PrimitiveComponent") _returnvalue_4 "None" true)
      (else
        (Physics|AddImpulse (Actor|GetComponentbyClass _array_element "/Script/Engine.CharacterMovementComponent") _returnvalue_4 true)))))

(fn ConstructionScript
  (Transformation|SetRelativeScale3D (Variables|Default|GetArrow) (/ "1.000000,1.000000,1.000000" (Transformation|GetActorScale3D))))