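; B_Virus is a collectable that adds to the player's collected data count when picked up.
; Its OnCollected function casts the collecting player's controller to B_PlayerController and increments CollectedData by one, doing nothing if the cast fails.
; The event graph holds only disabled placeholder events, and the construction script just calls the parent.
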(event EventBeginPlay
  (|CallParentFunction) ; This node is disabled and will not be called.\nDrag off pins to build functionality.
)

(event Collision|EventActorBeginOverlap
  (params (OtherActor :type Actor%20Object%20Reference))
  (|CallParentFunction OtherActor) ; This node is disabled and will not be called.\nDrag off pins to build functionality.
)

(event EventTick
  (params (DeltaSeconds :type Float%20%28single-precision%29))
  (|CallParentFunction DeltaSeconds) ; This node is disabled and will not be called.\nDrag off pins to build functionality.
)

(fn ConstructionScript
  (|CallParentFunction))

(fn OnCollected
  (params (Player :type B%20Player%20Object%20Reference))
  (bind _asb_player_controller (Utilities|Casting|CastToB_PlayerController (Pawn|GetController Player)))
  (Math|Integer|IncrementInt (Variables|/Game/Blueprints/B_PlayerController.B_PlayerController_C|GetcollectedData _asb_player_controller)))