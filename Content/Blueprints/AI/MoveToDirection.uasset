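; Behavior tree task that steers the controlled pawn straight toward the actor stored in the Target blackboard key.
; Each tick it feeds the unit direction to that actor into the CharacterMovementComponent as an input vector, with no navigation pathfinding.
; It then checks the distance, finishing with success within AcceptanceRadius or failure at or beyond FailRadius, and otherwise keeps running.
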(event EventReceiveExecuteAI
  (params (OwnerController :type AI%20Controller%20Object%20Reference) (ControlledPawn :type Pawn%20Object%20Reference)))

(event EventReceiveTickAI
  (params (OwnerController :type AI%20Controller%20Object%20Reference) (ControlledPawn :type Pawn%20Object%20Reference) (DeltaSeconds :type Float%20%28single-precision%29))
  (bind _returnvalue (Transformation|GetActorLocation ControlledPawn))
  (bind _target (Variables|Default|Gettarget))
  (bind _returnvalue_2 (AI|BehaviorTree|GetBlackboardValueasActor _target))
  (bind _returnvalue_3 (Transformation|GetActorLocation _returnvalue_2))
  (bind _returnvalue_4 (Math|Vector|Distance(Vector) _returnvalue _returnvalue_3))
  (Class|PawnMovementComponent|AddInputVector (Actor|GetComponentbyClass ControlledPawn "/Script/Engine.CharacterMovementComponent") (Math|Vector|GetUnitDirection(Vector) _returnvalue _returnvalue_3) false)
  (if (<= _returnvalue_4 (Variables|Default|GetacceptanceRadius))
    (AI|BehaviorTree|FinishExecute true)
    (elif (>= _returnvalue_4 (Variables|Default|GetfailRadius))
      (AI|BehaviorTree|FinishExecute false))))