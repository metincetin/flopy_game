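; DialogueManager is a component owned by B_PlayerController that runs dialogue sequences and switches the controller in and out of dialogue mode.
; SetDialogueDataList stores a list and shows its first entry through SetDialogueData, which broadcasts the change and begins dialogue if needed.
; NextDialogue advances the index through the list and ends dialogue past the last entry, clearing the active data but leaving the index unreset.
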(event EventBeginPlay)

(event EventTick
  (params (DeltaSeconds :type Float%20%28single-precision%29)))

(fn BeginDialogue
  (bind _asb_player_controller (Utilities|Casting|CastToB_PlayerController (Components|GetOwner)))
  (Default|EnterDialogue _asb_player_controller)
  (Variables|Default|SetIsInDialogueMode true))

(fn EndDialogue
  (bind _asb_player_controller (Utilities|Casting|CastToB_PlayerController (Components|GetOwner)))
  (Default|ExitDialogue _asb_player_controller)
  (Variables|Default|SetIsInDialogueMode false)
  (Variables|Default|SetActiveDialogueData ""))

(fn SetDialogueData
  (params (DialogueData :type Dialogue%20Data%20Structure))
  (Utilities|FlowControl|Sequence
    (:then_0
      (bind _output_get (Variables|Default|SetActiveDialogueData DialogueData))
      (Default|CallOnDialogueDataChanged _output_get))
    (:then_1
      (if (not (Variables|Default|GetIsInDialogueMode))
        (CallFunction|BeginDialogue)))))

(fn NextDialogue
  (bind _dialoguedatalist (Variables|Default|GetDialogueDataList))
  (bind _result (Math|Integer|IncrementInt (Variables|Default|GetCurrentDialogueIndex))
    (:%20%20
      (if (< _result (Utilities|Array|Length _dialoguedatalist))
        (CallFunction|SetDialogueData (Utilities|Array|Get(acopy) _dialoguedatalist _result))
        (else
          (CallFunction|EndDialogue))))))

(fn SetDialogueDataList
  (params (DialogueDataList :type Array%20of%20Dialogue%20Data%20Structures))
  (bind _output_get (Variables|Default|SetDialogueDataList DialogueDataList))
  (if (> (Utilities|Array|Length _output_get) 0)
    (CallFunction|SetDialogueData (Utilities|Array|Get(acopy) _output_get))))