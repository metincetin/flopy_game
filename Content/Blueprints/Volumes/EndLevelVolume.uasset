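; EndLevelVolume is a trigger volume that ends the level when the player enters it with enough collected data.
; On overlap it casts to B_Player and its B_PlayerController, then compares the controller's CollectedData to the volume's RequiredData.
; When the requirement is met, it fades the camera out, holds the fade, and after a short delay opens the referenced Level.
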(event EventBeginPlay)

(event Collision|EventActorBeginOverlap
  (params (OtherActor :type Actor%20Object%20Reference))
  (bind _asb_player (Utilities|Casting|CastToB_Player OtherActor))
  (bind _asb_player_controller (Utilities|Casting|CastToB_PlayerController (Pawn|GetController _asb_player)))
  (if (>= (Variables|/Game/Blueprints/B_PlayerController.B_PlayerController_C|GetcollectedData _asb_player_controller) (Variables|Default|GetrequiredData))
    (CameraFades|StartCameraFade :self (Game|GetPlayerCameraManager 0) :ToAlpha 1.0 :Duration 1.0 :bHoldWhenFinished true)
    (Utilities|FlowControl|Delay 1.0)
    (CallFunction|LoadLevel)))

(fn ConstructionScript)

(fn LoadLevel
  (Game|OpenLevel(byObjectReference) (Variables|Default|GetLevel)))