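; End-of-game volume that extends a parent level-loading volume to show an end screen before the level change.
; Its LoadLevel override hands off to the LoadLevelInternal event, which allows a latent Delay in the event graph.
; That event adds a B_End_UI widget to the first player's viewport, waits briefly, then calls the parent's LoadLevel.
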(event Custom|LoadLevelInternal
  (bind _returnvalue (UserInterface|CreateWidget "/Game/Blueprints/UI/B_End_UI.B_End_UI_C" (Game|GetPlayerController 0)))
  (UserInterface|Viewport|AddtoViewport _returnvalue 0)
  (Utilities|FlowControl|Delay 1.0)
  (|CallParentFunction))

(event EventBeginPlay
  (|CallParentFunction) ; This node is disabled and will not be called.\nDrag off pins to build functionality.
)

(event Collision|EventActorBeginOverlap
  (params (OtherActor :type Actor%20Object%20Reference))
  (|CallParentFunction OtherActor) ; This node is disabled and will not be called.\nDrag off pins to build functionality.
)

(event EventTick
  (params (DeltaSeconds :type Float%20%28single-precision%29)))

(fn ConstructionScript
  (|CallParentFunction))

(fn LoadLevel
  (CallFunction|LoadLevelInternal))